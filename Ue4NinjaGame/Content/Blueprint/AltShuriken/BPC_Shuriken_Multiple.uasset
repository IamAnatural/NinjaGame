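; Shuriken component for the "Multiple" effect that spawns extra shurikens in a fan around the player's facing.
; MultipleOnBeginPlay reads count and angle from a stats DataTable, then alternates positive and negative yaw offsets via FlipFlop, widening after each pair.
; ShurikenSpawn creates each BP_Shuriken at the player mesh's shuriken socket, passing on the effects minus one enum entry, likely Multiple itself to prevent recursive spawning.
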(fn `Multiple on Begin Play`
  (params (ShurikenEffects :type "Array of /Game/Blueprint/EShurikenEffects Enum"))
  (locals (DegreeMultiplier :type "Float (double-precision)" :default 1.0))
  (bind _returnvalue (`|GetDataTableRow` "/Game/Blueprint/Stats_DataTable.Stats_DataTable" "MultipleBaseCounter")
    (:`then`
      (for _ (range 2 (+ (`KismetMathLibrary.FTrunc` (break `/Game/Blueprint/Stats_Struct` _returnvalue)) 1))
        (bind _returnvalue_2 (`|GetDataTableRow` "/Game/Blueprint/Stats_DataTable.Stats_DataTable" "MultipleAngle")
          (:`then`
            (`/Engine/EditorBlueprintResources/StandardMacros.FlipFlop`
              (:`A`
                (`self.Shuriken Spawn` (`KismetMathLibrary.MakeRotator` 0.0 0.0 (* (break `/Game/Blueprint/Stats_Struct` _returnvalue_2) (`local.DegreeMultiplier`))) ShurikenEffects))
              (:`B`
                (`self.Shuriken Spawn` (`KismetMathLibrary.MakeRotator` 0.0 0.0 (* (* (break `/Game/Blueprint/Stats_Struct` _returnvalue_2) -1.0) (`local.DegreeMultiplier`))) ShurikenEffects)
                (`/Engine/EditorBlueprintResources/StandardMacros.IncrementFloat` (`local.DegreeMultiplier`))))))))))

(fn `Shuriken Spawn`
  (params (InputRotationOffset :type "Rotator Structure") (ShurikenEffects :type "Array of /Game/Blueprint/EShurikenEffects Enum"))
  (locals (Effects :type "Array of /Game/Blueprint/EShurikenEffects Enum"))
  (bind _returnvalue (`GameplayStatics.GetPlayerPawn` 0))
  ;[1 1 1] Spawn Projectile at Location
  (bind _output_get (set `local.Effects` ShurikenEffects))
  (`KismetArrayLibrary.Array_RemoveItem` _output_get "NewEnumerator4")
  (bind _asbp_base_pawn (cast `/Game/Blueprint/Bp_BasePawn` _returnvalue))
  (bind _returnvalue_2 (`|SpawnActorFromClass` "/Game/Blueprint/BP_Shuriken.BP_Shuriken_C" (`KismetMathLibrary.MakeTransform` (`SceneComponent.GetSocketLocation` (`Character.Mesh` _asbp_base_pawn) "Socket_Shuriken") (`KismetMathLibrary.ComposeRotators` InputRotationOffset (`Actor.K2_GetActorRotation` _returnvalue))) "AlwaysSpawn" "OverrideRootScale" null null))
  ;[1 1 1] Set Shuriken Component
  (`/Engine/EditorBlueprintResources/StandardMacros.IsValid` _returnvalue_2
    (:`Is Valid`
      (set `/Game/Blueprint/BP_Shuriken.Effects` (`local.Effects`) _returnvalue_2))))