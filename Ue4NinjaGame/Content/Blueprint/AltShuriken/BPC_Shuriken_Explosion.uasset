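; Actor component that gives a BP_Shuriken an explosion when it is destroyed.
; On construction it sizes the shuriken's RangeSphereExplosive from the ExplosionBaseRadius row of the stats data table.
; Before destruction it spawns a fire hit emitter scaled to that sphere's radius, then sends ExplosionBaseDmg from the same table to every overlapping BP_BaseEnemy via DamageInputMessage.
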(fn `Explosion_BeforeDestroy`
  (bind _returnvalue (`self.GetOwner`))
  (bind _asbp_shuriken (cast `/Game/Blueprint/BP_Shuriken` _returnvalue))
  (bind _rangesphere_explosive (`/Game/Blueprint/BP_Shuriken.RangeSphere_Explosive` _asbp_shuriken))
  (`GameplayStatics.SpawnEmitterAtLocation` "/Game/MarketPlace/AdvancedMagicFX12/particles/P_ky_hit_fire.P_ky_hit_fire" (`Actor.K2_GetActorLocation` _returnvalue) (struct) (* (1.0 1.0 1.0) (/ (`SphereComponent.GetScaledSphereRadius` _rangesphere_explosive) 175.0)))
  (for _array_element (`PrimitiveComponent.GetOverlappingActors` _rangesphere_explosive "/Game/Blueprint/BP_BaseEnnemy.BP_BaseEnemy_C")
    (bind _returnvalue_2 (`|GetDataTableRow` "/Game/Blueprint/Stats_DataTable.Stats_DataTable" "ExplosionBaseDmg")
      (:`then`
        (message `/Game/Blueprint/BPI_Damage.DamageInput` _array_element (break `/Game/Blueprint/Stats_Struct` _returnvalue_2) "NewEnumerator0")))))

(fn `Explosion_OnConstruction`
  (bind _asbp_shuriken (cast `/Game/Blueprint/BP_Shuriken` (`self.GetOwner`)))
  (bind _returnvalue (`|GetDataTableRow` "/Game/Blueprint/Stats_DataTable.Stats_DataTable" "ExplosionBaseRadius")
    (:`then`
      (`SphereComponent.SetSphereRadius` (`/Game/Blueprint/BP_Shuriken.RangeSphere_Explosive` _asbp_shuriken) (break `/Game/Blueprint/Stats_Struct` _returnvalue) true))))