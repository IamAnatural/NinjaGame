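; Poison cloud actor for the alt shuriken that repeatedly damages every enemy inside its sphere until its lifespan expires.
; The construction script reads radius and duration from a stats data table, sizing the sphere, scaling Niagara thickness and density to it, and setting the lifespan.
; From BeginPlay, a self-retriggering Delay event sends table-driven damage to overlapping BP_BaseEnemy actors at the table's tick interval.
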(event `self.ReceiveBeginPlay`
  (`self.DealPoisonDamage`))

(event `DealPoisonDamage`
  (bind _returnvalue (`|GetDataTableRow` "/Game/Blueprint/Stats_DataTable.Stats_DataTable" "PoisonBaseDmg")
    (:`then`
      (message `/Game/Blueprint/BPI_Damage.DamageInput` (`PrimitiveComponent.GetOverlappingActors` (`self.Sphere`) "/Game/Blueprint/BP_BaseEnnemy.BP_BaseEnemy_C") (break `/Game/Blueprint/Stats_Struct` _returnvalue) "NewEnumerator6")
      (bind _returnvalue_2 (`|GetDataTableRow` "/Game/Blueprint/Stats_DataTable.Stats_DataTable" "PoisonBaseTickTime")
        (:`then`
          (`KismetSystemLibrary.Delay` (break `/Game/Blueprint/Stats_Struct` _returnvalue_2))
          (`self.DealPoisonDamage`))))))

(fn `UserConstructionScript`
  (bind _returnvalue (/ (`SphereComponent.GetScaledSphereRadius` (`self.Sphere`)) 75.0))
  (bind _returnvalue_2 (`|GetDataTableRow` "/Game/Blueprint/Stats_DataTable.Stats_DataTable" "ShurikenPoisonRadius")
    (:`then`
      (`SphereComponent.SetSphereRadius` (`self.Sphere`) (break `/Game/Blueprint/Stats_Struct` _returnvalue_2) true)
      (`FXSystemComponent.SetFloatParameter` (`self.Niagara`) "Thickness" (* _returnvalue 1.0))
      (`FXSystemComponent.SetFloatParameter` (`self.Niagara`) "Density" (* _returnvalue 50.0))
      (bind _returnvalue_3 (`|GetDataTableRow` "/Game/Blueprint/Stats_DataTable.Stats_DataTable" "PoisonBaseDuration")
        (:`then`
          (`self.SetLifeSpan` (break `/Game/Blueprint/Stats_Struct` _returnvalue_3)))))))