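; A shuriken ability pickup variant that grants a randomly chosen effect: Stun, Pierce, Ricochet, Multiple, Explosive, Poison or Big.
; The Construction Script rolls the effect, selects its matching color and shuriken mesh, and tints the pickup particles before running the parent script.
; Overlap handling is left entirely to the parent class.
; Because the roll happens during construction, the effect can change whenever that script reruns.
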(event `self.ReceiveActorBeginOverlap`
  (params (OtherActor :type "Actor Object Reference"))
  (`parent.ReceiveActorBeginOverlap` OtherActor))

(fn `UserConstructionScript`
  (bind _output_get (set `self.ShurikenEffect` (`KismetArrayLibrary.Array_Random` (`|MakeArray` "NewEnumerator1" "NewEnumerator2" "NewEnumerator3" "NewEnumerator4" "NewEnumerator5" "NewEnumerator6" "NewEnumerator7" :!type "/Game/Blueprint/EShurikenEffects Enum"))))
  (bind _output_get_2 (set `self.ObjectColor` (select `/Game/Blueprint/EShurikenEffects` _output_get :`NewEnumerator1` (struct :`G` 2.0 :`B` 1.945447 :`A` 1.0) :`NewEnumerator2` (struct :`R` 1.0 :`G` 0.9575 :`A` 1.0) :`NewEnumerator3` (struct :`R` 1.764504 :`B` 3.0 :`A` 1.0) :`NewEnumerator4` (struct :`R` 0.997333 :`G` 1.0 :`B` 0.953415 :`A` 1.0) :`NewEnumerator5` (struct :`R` 5.0 :`B` 0.11503 :`A` 1.0) :`NewEnumerator6` (struct :`R` 0.19523 :`G` 3.0 :`A` 1.0) :`NewEnumerator7` (struct :`G` 0.259696 :`B` 3.0 :`A` 1.0) :!type "LinearColor Structure")))
  (`StaticMeshComponent.SetStaticMesh` (`self.Cube`) (select `/Game/Blueprint/EShurikenEffects` _output_get :`NewEnumerator1` "/Game/Blueprint/AltShuriken/Mesh/SM_Shuriken_Stun.SM_Shuriken_Stun" :`NewEnumerator2` "/Game/Blueprint/AltShuriken/Mesh/SM_Shuriken_Pierce.SM_Shuriken_Pierce" :`NewEnumerator3` "/Game/Blueprint/AltShuriken/Mesh/SM_Shuriken_Ricochet.SM_Shuriken_Ricochet" :`NewEnumerator4` "/Game/Blueprint/AltShuriken/Mesh/SM_Shuriken_Multiple.SM_Shuriken_Multiple" :`NewEnumerator5` "/Game/Blueprint/AltShuriken/Mesh/SM_Shuriken_Explosion.SM_Shuriken_Explosion" :`NewEnumerator6` "/Game/Blueprint/AltShuriken/Mesh/SM_Shuriken_Poison.SM_Shuriken_Poison" :`NewEnumerator7` "/Game/Blueprint/AltShuriken/Mesh/SM_Shuriken_Big.SM_Shuriken_Big" :!type "StaticMesh Object Reference"))
  (`FXSystemComponent.SetColorParameter` (`self.PickUpEffect`) "Color" _output_get_2)
  (`parent.UserConstructionScript`))