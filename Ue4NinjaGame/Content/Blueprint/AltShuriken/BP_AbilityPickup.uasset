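; Timed pickup actor that grants a shuriken effect to any BP_BasePawn that overlaps it.
; The construction script tints the cube with ObjectColor and sets the actor's lifespan from the PickUpDuration row of a stats data table.
; On overlap, it plays a buff sound, passes its ShurikenEffect to the pawn through AddShurikenEffect, then destroys itself.
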(event `self.ReceiveActorBeginOverlap`
  (params (OtherActor :type "Actor Object Reference"))
  (`self.GiveAbilityToPlayer` OtherActor))

(fn `GiveAbilityToPlayer`
  (params (PlayerActor :type "Object Object Reference"))
  (bind _asbp_base_pawn (cast `/Game/Blueprint/Bp_BasePawn` PlayerActor))
  (`GameplayStatics.PlaySoundAtLocation` "/Game/SFX/ultimate_Medieval_Combat_SFX/Magic_SFX_Pro/Wavs/Buffs/Buff_18.Buff_18" (`SceneComponent.K2_GetComponentLocation` (`self.DefaultSceneRoot`)) (struct) 1.0 1.0 0.0 null null null)
  (`/Game/Blueprint/Bp_BasePawn.AddShurikenEffect` _asbp_base_pawn (`self.ShurikenEffect`))
  (`self.K2_DestroyActor`))

(fn `UserConstructionScript`
  (`MeshComponent.SetVectorParameterValueOnMaterials` (`self.Cube`) "Color" (`KismetMathLibrary.Conv_LinearColorToVector` (`self.ObjectColor`)))
  (bind _returnvalue (`|GetDataTableRow` "/Game/Blueprint/Stats_DataTable.Stats_DataTable" "PickUpDuration")
    (:`then`
      (`self.SetLifeSpan` (break `/Game/Blueprint/Stats_Struct` _returnvalue)))))