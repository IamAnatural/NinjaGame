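; Shuriken component that makes a shuriken ricochet to another nearby enemy before it is destroyed on an enemy hit.
; On BeginPlay it sizes the shuriken's RangeSphere from the stats DataTable, then on hit searches that sphere for the BP_BaseEnemy nearest the one struck.
; It spawns a new shuriken aimed at that enemy with a table-driven lifespan.
; The new shuriken gets Ricochet and Explosion components with a decremented counter, or only Base at zero.
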(event `self.ReceiveBeginPlay`
  (`parent.ReceiveBeginPlay`)
  (bind _returnvalue (`|GetDataTableRow` "/Game/Blueprint/Stats_DataTable.Stats_DataTable" "ShurikenRicochetRange")
    (:`then`
      (`SphereComponent.SetSphereRadius` (`/Game/Blueprint/BP_Shuriken.RangeSphere` (`self.ShurikenActor`)) (break `/Game/Blueprint/Stats_Struct` _returnvalue) true))))

(fn `BeforeDestroyOnEnemy`
  (params (Actor :type "Actor Object Reference"))
  (bind _returnvalue (`Actor.K2_GetActorLocation` Actor))
  (bind (_actorisvalid _actorlocation) (`self.ToNearestInRange` Actor))
  (if _actorisvalid
    ;[1 1 1] Spawn Projectile at Location
    (bind _returnvalue_2 (`|SpawnActorFromClass` "/Game/Blueprint/BP_Shuriken.BP_Shuriken_C" (`KismetMathLibrary.MakeTransform` _returnvalue (`KismetMathLibrary.FindLookAtRotation` _returnvalue _actorlocation)) "AlwaysSpawn" "OverrideRootScale" null null))
    ;[1 1 1] Set Shuriken Component
    (`/Engine/EditorBlueprintResources/StandardMacros.IsValid` _returnvalue_2
      (:`Is Valid`
        (if (== (`self.RicochetCounter`) 0)
          (`|AddComponentByClass` _returnvalue_2 "/Game/Blueprint/AltShuriken/BPC_Shuriken_Base.BPC_Shuriken_Base_C")
          (else
            (bind _returnvalue_3 (`|AddComponentByClass` _returnvalue_2 "BPC_Shuriken_Ricochet_C"))
            (`|AddComponentByClass` _returnvalue_2 "/Game/Blueprint/AltShuriken/BPC_Shuriken_Explosion.BPC_Shuriken_Explosion_C")
            (set `/Game/Blueprint/AltShuriken/BPC_Shuriken_Ricochet.RicochetCounter` (- (`self.RicochetCounter`) 1) _returnvalue_3)))
        (bind _returnvalue_4 (`|GetDataTableRow` "/Game/Blueprint/Stats_DataTable.Stats_DataTable" "ShurikenBaseLifespan")
          (:`then`
            (`Actor.SetLifeSpan` _returnvalue_2 (break `/Game/Blueprint/Stats_Struct` _returnvalue_4)))))))
  (`parent.BeforeDestroyOnEnemy` Actor))

(fn `ToNearestInRange`
  (params (Actor :type "Actor Object Reference"))
  (returns (ActorIsValid :type Boolean) (ActorLocation :type "Vector Structure"))
  (locals (NearestMonsterDistance :type "Float (double-precision)" :default 1000.0) (NearestMonster :type "Actor Object Reference"))
  (bind _nearestmonster (`local.NearestMonster`))
  (for _array_element (`PrimitiveComponent.GetOverlappingActors` (`/Game/Blueprint/BP_Shuriken.RangeSphere` (`self.ShurikenActor`)) "/Game/Blueprint/BP_BaseEnnemy.BP_BaseEnemy_C")
    (bind _returnvalue (`KismetMathLibrary.Vector_Distance` (`Actor.K2_GetActorLocation` _array_element) (`Actor.K2_GetActorLocation` Actor)))
    (if (and (< _returnvalue (`local.NearestMonsterDistance`)) (!= _array_element Actor))
      (set `local.NearestMonsterDistance` _returnvalue)
      (set `local.NearestMonster` _array_element)))
  (`/Engine/EditorBlueprintResources/StandardMacros.IsValid` _nearestmonster
    (:`Is Valid`
      (return true (`Actor.K2_GetActorLocation` _nearestmonster)))
    (:`Is Not Valid`
      (return false (0.0 0.0 0.0)))))