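; Base behavior component for BP_Shuriken projectiles, handling lifespan, impacts and damage.
; On BeginPlay it sets lifespan from a stats data table, then binds mesh overlap and actor hit events.
; Overlaps with actors other than the player deal table-driven or overridden damage through BPI_Damage, then destroy the shuriken.
; Hits just destroy it, with separate BeforeDestroy and Destroy functions serving as hooks for each case.
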(event `self.ReceiveBeginPlay`
  (bind _returnvalue (`self.GetOwner`))
  (bind _asbp_shuriken (cast `/Game/Blueprint/BP_Shuriken` _returnvalue))
  (set `self.ShurikenActor` _asbp_shuriken)
  (bind _returnvalue_2 (`|GetDataTableRow` "/Game/Blueprint/Stats_DataTable.Stats_DataTable" "ShurikenBaseLifespan")
    (:`then`
      (`Actor.SetLifeSpan` (`self.ShurikenActor`) (break `/Game/Blueprint/Stats_Struct` _returnvalue_2))
      (add `PrimitiveComponent.OnComponentBeginOverlap` (`/Game/Blueprint/BP_Shuriken.ProjectileMesh` _asbp_shuriken) (delegate `ShurikenOverlapped`))
      (add `Actor.OnActorHit` _returnvalue (delegate `Actor_Hit`)))))

(event `Actor_Hit`
  (params (SelfActor :type "Actor Object Reference") (OtherActor :type "Actor Object Reference") (NormalImpulse :type "Vector Structure") (Hit :type "HitResult Structure (by ref)"))
  (`self.BeforeDestroyOnHit` OtherActor Hit)
  (`self.DestroyOnHit`))

(event `ShurikenOverlapped`
  (params (OverlappedComponent :type "PrimitiveComponent Object Reference") (OtherActor :type "Actor Object Reference") (OtherComp :type "PrimitiveComponent Object Reference") (OtherBodyIndex :type Integer) (bFromSweep :type Boolean) (SweepResult :type "HitResult Structure (by ref)"))
  (if (and (!= OtherActor (`GameplayStatics.GetPlayerPawn` 0)) (!= OtherActor "/Game/Blueprint/BP_Shuriken.BP_Shuriken"))
    (`self.BeforeDestroyOnEnemy` OtherActor)
    (`self.DestroyOnEnemy`)))

(fn `ApplyDamage`
  (params (Actor :type "Actor Object Reference") (AttackType :type "/Game/Blueprint/EShurikenEffects Enum" :default "NewEnumerator0") (OverwriteDamage :type "Float (double-precision)"))
  (`/Engine/EditorBlueprintResources/StandardMacros.IsValid` Actor
    (:`Is Valid`
      (bind _returnvalue (`|GetDataTableRow` "/Game/Blueprint/Stats_DataTable.Stats_DataTable" "ShurikenBaseDmg")
        (:`then`
          (if (`KismetSystemLibrary.DoesImplementInterface` Actor "/Game/Blueprint/BPI_Damage.BPI_Damage_C")
            (message `/Game/Blueprint/BPI_Damage.DamageInput` Actor (select `bool` (!= OverwriteDamage 0.0) :`false` (break `/Game/Blueprint/Stats_Struct` _returnvalue) :`true` OverwriteDamage) AttackType)))))))

(fn `BeforeDestroyOnEnemy`
  (params (Actor :type "Actor Object Reference"))
  (`self.ApplyDamage` Actor))

(fn `BeforeDestroyOnHit`
  (params (Actor :type "Actor Object Reference") (Hit :type "HitResult Structure")))

(fn `DestroyOnEnemy`
  (`Actor.K2_DestroyActor` (`self.GetOwner`)))

(fn `DestroyOnHit`
  (`Actor.K2_DestroyActor` (`self.GetOwner`)))