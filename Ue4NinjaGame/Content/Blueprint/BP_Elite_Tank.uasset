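; BP_Elite_Tank is an elite tank variant with scaled health, its own score multiplier and an ability drop.
; After the parent construction script, it multiplies Health by a stats data table value, then reads ScoreMultiplier from a second row.
; The LogicOnDestroy override spawns a BP_AbilityPickUp_Random at the capsule's location before calling the parent logic.
; The event graph adds no active behavior.
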(fn `LogicOnDestroy`
  ;[1 1 1] Spawn AbilityPickUp Randomly
  (`|SpawnActorFromClass` "/Game/Blueprint/AltShuriken/BP_AbilityPickUp_Random.BP_AbilityPickUp_Random_C" (`KismetMathLibrary.MakeTransform` (`SceneComponent.K2_GetComponentLocation` (`self.CapsuleComponent`)) (struct) (1.0 1.0 1.0)) "Undefined" "OverrideRootScale" null null)
  (`parent.LogicOnDestroy`)
  (return))

(fn `UserConstructionScript`
  (`parent.UserConstructionScript`)
  (bind _returnvalue (`|GetDataTableRow` "/Game/Blueprint/Stats_DataTable.Stats_DataTable" "EliteHealthMultiplier")
    (:`then`
      (set `self.Health` (* (break `/Game/Blueprint/Stats_Struct` _returnvalue) (`self.Health`)))
      (bind _returnvalue_2 (`|GetDataTableRow` "/Game/Blueprint/Stats_DataTable.Stats_DataTable" "EliteScoreMultiplier")
        (:`then`
          (set `self.ScoreMultiplier` (break `/Game/Blueprint/Stats_Struct` _returnvalue_2)))))))