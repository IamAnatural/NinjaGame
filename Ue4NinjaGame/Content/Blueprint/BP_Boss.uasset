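; Boss enemy that fires projectiles at player pawns, with health and score multipliers over its parent class.
; Entering AttackSphere stops movement and starts a timeline-driven yaw turn toward the player; after a windup it fires, resumes moving, then retries after cooldown.
; On destruction it spawns base enemies at random navigable points and random ability pickups around its mesh.
; Timings, multipliers and spawn counts come from a stats DataTable.
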(event `ShootProjectile`
  (bind (_returnvalue_location _returnvalue_rotation) (`KismetMathLibrary.BreakTransform` (`SceneComponent.K2_GetComponentToWorld` (`self.ProjectileSpawnLocation`))))
  ;[1 1 1] Shoot Projectile
  (if (and (> (`KismetArrayLibrary.Array_Length` (`PrimitiveComponent.GetOverlappingActors` (`self.AttackSphere`) "/Game/Blueprint/Bp_BasePawn.BP_BasePawn_C")) 0) (not (`self.InCooldown`)))
    (set `/Game/Monsters/Animation/AnimBP_Monster.Moving` false (`self.AnimInstance`))
    (`NavMovementComponent.StopActiveMovement` (`self.CharacterMovement`))
    (set `self.InCooldown` true)
    (set `/Game/Monsters/Animation/AnimBP_Monster.Attacking` true (`self.AnimInstance`))
    (`self.StartLookAtPlayer`)
    (bind _returnvalue (`|GetDataTableRow` "/Game/Blueprint/Stats_DataTable.Stats_DataTable" "MonsterAttackSpeed")
      (:`then`
        (`KismetSystemLibrary.Delay` (break `/Game/Blueprint/Stats_Struct` _returnvalue)) ; Time of attack
        (`|SpawnActorFromClass` "/Game/Blueprint/BP_BossProjectile.BP_BossProjectile_C" (`KismetMathLibrary.MakeTransform` _returnvalue_location _returnvalue_rotation) "Undefined" "OverrideRootScale" null null)
        (`self.StopLookAtPlayer`)
        (`self.MoveTo`)
        (bind _returnvalue_2 (`|GetDataTableRow` "/Game/Blueprint/Stats_DataTable.Stats_DataTable" "BossAbilityCooldown")
          (:`then`
            (`KismetSystemLibrary.Delay` (break `/Game/Blueprint/Stats_Struct` _returnvalue_2)) ; Next Shot Cooldown
            (set `self.InCooldown` false)
            (`self.ShootProjectile`)))))))

(event `self.AttackSphere.OnComponentBeginOverlap`
  (params (OverlappedComponent :type "PrimitiveComponent Object Reference") (OtherActor :type "Actor Object Reference") (OtherComp :type "PrimitiveComponent Object Reference") (OtherBodyIndex :type Integer) (bFromSweep :type Boolean) (SweepResult :type "HitResult Structure (by ref)"))
  ;[1 1 1] On Overlap AttackSpeed
  (`self.ShootProjectile`))

(event `StartLookAtPlayer`
  (bind (_returnvalue_roll _returnvalue_pitch _returnvalue_yaw) (`KismetMathLibrary.BreakRotator` (`KismetMathLibrary.FindLookAtRotation` (`SceneComponent.K2_GetComponentLocation` (`self.CapsuleComponent`)) (`self.K2_GetActorLocation` (`GameplayStatics.GetPlayerPawn` 0)))))
  ;[1 1 1] Look at Player
  (`Timeline|LookAtPlayer` :!label _label
    (:`Update`
      (`self.K2_SetActorRotation` (`KismetMathLibrary.MakeRotator` 0.0 0.0 _returnvalue_yaw)))))

(event `StopLookAtPlayer`
  ;[1 1 1] Look at Player
  (goto _label :!via `Stop`))

(fn `LogicOnDestroy`
  (bind _spawnsphere (`self.SpawnSphere`))
  ;[1 1 1] Spawn Enemies
  (bind _returnvalue (`|GetDataTableRow` "/Game/Blueprint/Stats_DataTable.Stats_DataTable" "BossEnemySpawnNumber")
    (:`then`
      (for _ (range 1 (+ (`KismetMathLibrary.FTrunc` (break `/Game/Blueprint/Stats_Struct` _returnvalue)) 1))
        (bind _randomlocation (`NavigationSystemV1.K2_GetRandomLocationInNavigableRadius` (`SceneComponent.K2_GetComponentLocation` _spawnsphere) (`SphereComponent.GetScaledSphereRadius` _spawnsphere) null null))
        (`|SpawnActorFromClass` "/Game/Blueprint/BP_BaseEnnemy.BP_BaseEnemy_C" (`KismetMathLibrary.MakeTransform` _randomlocation) "Undefined" "OverrideRootScale" null null))
      ;[1 1 1] Spawn AbilityPickUp Randomly
      (bind _returnvalue_2 (`|GetDataTableRow` "/Game/Blueprint/Stats_DataTable.Stats_DataTable" "BossAbilitySpawnNumber")
        (:`then`
          (for _index (range 1 (+ (`KismetMathLibrary.FTrunc` (break `/Game/Blueprint/Stats_Struct` _returnvalue_2)) 1))
            (`|SpawnActorFromClass` "/Game/Blueprint/AltShuriken/BP_AbilityPickUp_Random.BP_AbilityPickUp_Random_C" (`KismetMathLibrary.MakeTransform` (+ (select `int` _index :`0` (0.0 0.0 0.0) :`1` (200.0 0.0 0.0) :`2` (-200.0 0.0 0.0) :`3` (0.0 -200.0 0.0) :!type "Vector Structure") (`SceneComponent.K2_GetComponentLocation` (`self.Mesh`)))) "Undefined" "OverrideRootScale" null null))
          (`parent.LogicOnDestroy`)
          (return))))))

(fn `SetBaseHealthMath`
  (returns (ReturnValue :type "Float (double-precision)"))
  (bind _returnvalue (`parent.SetBaseHealthMath`))
  (bind _returnvalue_2 (`|GetDataTableRow` "/Game/Blueprint/Stats_DataTable.Stats_DataTable" "BossHealthMultiplier")
    (:`then`
      (return (* _returnvalue (break `/Game/Blueprint/Stats_Struct` _returnvalue_2))))))

(fn `UserConstructionScript`
  (`parent.UserConstructionScript`)
  (bind _returnvalue (`|GetDataTableRow` "/Game/Blueprint/Stats_DataTable.Stats_DataTable" "BossScoreMultiplier")
    (:`then`
      (set `self.ScoreMultiplier` (break `/Game/Blueprint/Stats_Struct` _returnvalue))
      (set `self.DeathEmitter` "/Game/MarketPlace/AdvancedMagicFX12/particles/P_ky_hit.P_ky_hit"))))