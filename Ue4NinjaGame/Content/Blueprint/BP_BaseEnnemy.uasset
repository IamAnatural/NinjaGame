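; Base enemy that chases the first player and attacks with a headbump on reaching them.
; A looping AI MoveTo drives AnimBP_Monster flags, then after a short wind-up damages the player if overlapping AttackBox.
; Dmg lowers Health, destroying the enemy with a particle burst at zero, or flagging a hit reaction and stopping movement.
; The Recovered event restarts the chase.
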(event `self.ReceiveBeginPlay`
  (bind _asanim_bp_monster (cast `/Game/Monsters/Animation/AnimBP_Monster` (`SkeletalMeshComponent.GetAnimInstance` (`self.Mesh`))))
  (set `self.AnimInstance` _asanim_bp_monster)
  (`self.MoveTo`))

(event `MoveTo`
  (bind _returnvalue (`GameplayStatics.GetPlayerPawn` 0))
  (bind _animinstance (`self.AnimInstance`))
  ;[1 1 1] Move to logic
  (set `/Game/Monsters/Animation/AnimBP_Monster.Moving` true (`self.AnimInstance`))
  (`|AIMoveTo` self (`self.K2_GetActorLocation` _returnvalue) _returnvalue 0.0
    (:`OnSuccess`
      (set `/Game/Monsters/Animation/AnimBP_Monster.Moving` false _animinstance)
      (set `/Game/Monsters/Animation/AnimBP_Monster.Attacking` true _animinstance)
      (`KismetSystemLibrary.Delay` 0.5) ; Time of attack
      (if (`PrimitiveComponent.IsOverlappingActor` (`self.AttackBox`) _returnvalue)
        (message `/Game/Blueprint/BPI_Damage.ReceiveDmg` (`GameplayStatics.GetPlayerPawn` 0) (`self.Damage`) "Headbump"))
      (`self.MoveTo`))
    (:`OnFail`
      (set `/Game/Monsters/Animation/AnimBP_Monster.Moving` false _animinstance))))

(event `/Game/Blueprint/BPI_Damage.ReceiveDmg`
  (params (Damages :type "Float (single-precision)") (AttackType :type String))
  ;[1 1 1] Receive dmg
  (bind _output_get (set `self.Health` (- (`self.Health`) Damages)))
  (if (<= _output_get 0.0)
    (`GameplayStatics.SpawnEmitterAtLocation` "/Game/MarketPlace/AdvancedMagicFX12/particles/P_ky_hit_dark.P_ky_hit_dark" (`SceneComponent.K2_GetComponentLocation` (`self.CapsuleComponent`)))
    (`self.K2_DestroyActor`)
    (else
      (set `/Game/Monsters/Animation/AnimBP_Monster.IsHit` true (`self.AnimInstance`))
      (`NavMovementComponent.StopActiveMovement` (`self.CharacterMovement`)))))

(event `Recovered`
  ;[1 1 1] Receive dmg
  (`self.MoveTo`))

(fn `UserConstructionScript`)