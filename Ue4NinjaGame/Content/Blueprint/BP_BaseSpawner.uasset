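; Enemy spawner that runs endless, self-rescheduling loops for normal enemies, random Quick or Tank elites, and bosses.
; Each picks a navigable point in SpawnSphere, retrying recursively while inside BlockShpere.
; Normal spawns start immediately, while elites and bosses first wait their data-table delay.
; Repeat delays pass through SpawnRateMaths, whose formula divides by a time-growing, capped divider tuned from the table at construction.
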(event `self.ReceiveBeginPlay`
  (`self.SpawnUnit`)
  (`|ExecutionSequence`
    (:`then_0`
      (bind _returnvalue (`|GetDataTableRow` "/Game/Blueprint/Stats_DataTable.Stats_DataTable" "EliteBaseSpawnRate")
        (:`then`
          (`KismetSystemLibrary.Delay` (break `/Game/Blueprint/Stats_Struct` _returnvalue)) ; Spawn Time Rate
          (`self.SpawnElite`))))
    (:`then_1`
      (bind _returnvalue_2 (`|GetDataTableRow` "/Game/Blueprint/Stats_DataTable.Stats_DataTable" "BossSpawnRate")
        (:`then`
          (`KismetSystemLibrary.Delay` (break `/Game/Blueprint/Stats_Struct` _returnvalue_2)) ; Spawn Time Rate
          (`self.SpawnBoss`))))))

(event `SpawnUnit`
  (bind _spawn_sphere (`self.Spawn_Sphere`))
  (bind _block_shpere (`self.Block_Shpere`))
  ;[1 1 1] Spawn Normal Unit
  (bind _randomlocation (`NavigationSystemV1.K2_GetRandomLocationInNavigableRadius` (`SceneComponent.K2_GetComponentLocation` _spawn_sphere) (`SphereComponent.GetScaledSphereRadius` _spawn_sphere) null null))
  (if (> (`KismetMathLibrary.Vector_Distance` _randomlocation (`SceneComponent.K2_GetComponentLocation` _block_shpere)) (`SphereComponent.SphereRadius` _block_shpere))
    (`|SpawnActorFromClass` "/Game/Blueprint/BP_BaseEnnemy.BP_BaseEnemy_C" (`KismetMathLibrary.MakeTransform` _randomlocation) "Undefined" "OverrideRootScale" null null)
    (bind _returnvalue (`|GetDataTableRow` "/Game/Blueprint/Stats_DataTable.Stats_DataTable" "MonsterBaseSpawnrate")
      (:`then`
        (`KismetSystemLibrary.Delay` (`self.SpawnRateMaths` (break `/Game/Blueprint/Stats_Struct` _returnvalue))) ; Spawn Time Rate
        (`self.SpawnUnit`)))
    (else
      (`self.SpawnUnit`))))

(event `SpawnElite`
  (bind _block_shpere (`self.Block_Shpere`))
  (bind _spawn_sphere (`self.Spawn_Sphere`))
  ;[1 1 1] Spawn Elite
  (bind _randomlocation (`NavigationSystemV1.K2_GetRandomLocationInNavigableRadius` (`SceneComponent.K2_GetComponentLocation` _spawn_sphere) (`SphereComponent.GetScaledSphereRadius` _spawn_sphere) null null))
  (if (> (`KismetMathLibrary.Vector_Distance` _randomlocation (`SceneComponent.K2_GetComponentLocation` _block_shpere)) (`SphereComponent.SphereRadius` _block_shpere))
    (if (`KismetMathLibrary.RandomBool`)
      (`|SpawnActorFromClass` "/Game/Blueprint/BP_Elite_Quick.BP_Elite_Quick_C" (`KismetMathLibrary.MakeTransform` _randomlocation) "Undefined" "OverrideRootScale" null null)
      (else
        (`|SpawnActorFromClass` "/Game/Blueprint/BP_Elite_Tank.BP_Elite_Tank_C" (`KismetMathLibrary.MakeTransform` _randomlocation) "Undefined" "OverrideRootScale" null null)))
    (bind _returnvalue (`|GetDataTableRow` "/Game/Blueprint/Stats_DataTable.Stats_DataTable" "EliteBaseSpawnRate")
      (:`then`
        (`KismetSystemLibrary.Delay` (`self.SpawnRateMaths` (break `/Game/Blueprint/Stats_Struct` _returnvalue))) ; Spawn Time Rate
        (`self.SpawnElite`)))
    (else
      (`self.SpawnElite`))))

(event `SpawnBoss`
  (bind _spawn_sphere (`self.Spawn_Sphere`))
  (bind _block_shpere (`self.Block_Shpere`))
  ;[1 1 1] Spawn Boss
  (bind _randomlocation (`NavigationSystemV1.K2_GetRandomLocationInNavigableRadius` (`SceneComponent.K2_GetComponentLocation` _spawn_sphere) (`SphereComponent.GetScaledSphereRadius` _spawn_sphere) null null))
  (if (> (`KismetMathLibrary.Vector_Distance` _randomlocation (`SceneComponent.K2_GetComponentLocation` _block_shpere)) (`SphereComponent.SphereRadius` _block_shpere))
    (`|SpawnActorFromClass` "/Game/Blueprint/BP_Boss.BP_Boss_C" (`KismetMathLibrary.MakeTransform` _randomlocation) "Undefined" "OverrideRootScale" null null)
    (bind _returnvalue (`|GetDataTableRow` "/Game/Blueprint/Stats_DataTable.Stats_DataTable" "BossSpawnRate")
      (:`then`
        (`KismetSystemLibrary.Delay` (`self.SpawnRateMaths` (break `/Game/Blueprint/Stats_Struct` _returnvalue))) ; Spawn Time Rate
        (`self.SpawnBoss`)))
    (else
      (`self.SpawnBoss`))))

(fn `UserConstructionScript`
  (bind _returnvalue (`|GetDataTableRow` "/Game/Blueprint/Stats_DataTable.Stats_DataTable" "SpawnRateDividerIncreaseRate")
    (:`then`
      (set `self.DifficultyIncreaseRate` (break `/Game/Blueprint/Stats_Struct` _returnvalue))
      (bind _returnvalue_2 (`|GetDataTableRow` "/Game/Blueprint/Stats_DataTable.Stats_DataTable" "SpawnRateDividerIncreaseAmount")
        (:`then`
          (set `self.SpawnRateIncrement` (break `/Game/Blueprint/Stats_Struct` _returnvalue_2))
          (bind _returnvalue_3 (`|GetDataTableRow` "/Game/Blueprint/Stats_DataTable.Stats_DataTable" "SpawnRateDividerCAP")
            (:`then`
              (set `self.SpawnRateDividerCAP` (break `/Game/Blueprint/Stats_Struct` _returnvalue_3)))))))))