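; BP_Elite_Quick is an elite enemy variant that spawns a group of BP_BaseEnemy when its destroy logic runs.
; Construction reads its score multiplier from the stats data table.
; LogicOnDestroy reads the EliteSummonerSpawnNumber row, spawns that many enemies at random navigable points within SpawnSphere's radius, then calls the parent logic, which is skipped if the row is missing.
; Base health math defers entirely to the parent.
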(fn `LogicOnDestroy`
  (bind _spawnsphere (`self.SpawnSphere`))
  (bind _returnvalue (`|GetDataTableRow` "/Game/Blueprint/Stats_DataTable.Stats_DataTable" "EliteSummonerSpawnNumber")
    (:`then`
      (for _ (range 1 (+ (`KismetMathLibrary.FTrunc` (break `/Game/Blueprint/Stats_Struct` _returnvalue)) 1))
        (bind _randomlocation (`NavigationSystemV1.K2_GetRandomLocationInNavigableRadius` (`SceneComponent.K2_GetComponentLocation` _spawnsphere) (`SphereComponent.GetScaledSphereRadius` _spawnsphere) null null))
        (`|SpawnActorFromClass` "/Game/Blueprint/BP_BaseEnnemy.BP_BaseEnemy_C" (`KismetMathLibrary.MakeTransform` _randomlocation) "Undefined" "OverrideRootScale" null null))
      (`parent.LogicOnDestroy`)
      (return))))

(fn `SetBaseHealthMath`
  (returns (ReturnValue :type "Float (double-precision)"))
  (bind _returnvalue (`parent.SetBaseHealthMath`))
  (return _returnvalue))

(fn `UserConstructionScript`
  (`parent.UserConstructionScript`)
  (bind _returnvalue (`|GetDataTableRow` "/Game/Blueprint/Stats_DataTable.Stats_DataTable" "EliteScoreMultiplier")
    (:`then`
      (set `self.ScoreMultiplier` (break `/Game/Blueprint/Stats_Struct` _returnvalue)))))