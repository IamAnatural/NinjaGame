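; Player character for a cursor-aimed action game, with melee and spin attacks, shuriken throws, a teleport dash and wheel zoom.
; Input triggers AnimBP_Base, while melee and spin events toggle hit volumes, using HittedActor to prevent repeat hits.
; Shurikens inherit the active effects list, and dashes line-trace to stop at static geometry.
; Stats come from a data table, and a UI_Base widget shows health, score, timer and game over.
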(event `InputAction|Primary`
  (params (Key :type "Key Structure"))
  ;[1 0.3906 0.3906] Melee Attack
  (:`Pressed`
    (bind _asanim_bp_base (cast `/Game/Blueprint/AnimBP_Base` (`SkeletalMeshComponent.GetAnimInstance` (`self.Mesh`))))
    (`/Game/Blueprint/AnimBP_Base.MeleeAttack` _asanim_bp_base)))

(event `SpinStart`
  ;[1 0.3906 0.3906] Melee Attack
  (`KismetArrayLibrary.Array_Clear` (`self.HittedActor`))
  (`PrimitiveComponent.SetCollisionEnabled` (`self.SpinCapsule`) "QueryOnly"))

(event `InputAxis|Forward`
  (params (AxisValue :type "Float (single-precision)"))
  ;[1 1 1] Player Movement
  (`self.AddMovementInput` (1.0 0.0 0.0) AxisValue))

(event `InputAction|Secondary`
  (params (Key :type "Key Structure"))
  ;[1 0.9448 0.3267] Throw Shuriken
  (:`Pressed`
    (bind _asanim_bp_base (cast `/Game/Blueprint/AnimBP_Base` (`SkeletalMeshComponent.GetAnimInstance` (`self.Mesh`))))
    (set `/Game/Blueprint/AnimBP_Base.ShurikenThrow` true _asanim_bp_base)))

(event `SpinEnd`
  ;[1 0.3906 0.3906] Melee Attack
  (`PrimitiveComponent.SetCollisionEnabled` (`self.SpinCapsule`) "NoCollision"))

(event `InputAxis|Right`
  (params (AxisValue :type "Float (single-precision)"))
  ;[1 1 1] Player Movement
  (`self.AddMovementInput` (0.0 1.0 0.0) AxisValue))

(event `InputAction|Dash`
  (params (Key :type "Key Structure"))
  ;[1 1 1] Dash
  (:`Pressed`
    (`self.Dash` :!label _label)))

(event `MeleeAttack`
  ;[1 0.3906 0.3906] Melee Attack
  (`KismetArrayLibrary.Array_Clear` (`self.HittedActor`))
  (`PrimitiveComponent.SetCollisionEnabled` (`self.MeleeBox`) "QueryOnly")
  (`KismetSystemLibrary.Delay` 0.0)
  (`PrimitiveComponent.SetCollisionEnabled` (`self.MeleeBox`) "NoCollision"))

(event `InputAction|Jump`
  (params (Key :type "Key Structure"))
  ;[1 1 1] Dash
  (:`Pressed`
    (goto _label)))

(event `Throw`
  ;[1 0.9448 0.3267] Throw Shuriken
  ;;[1 1 1] Spawn Projectile at location
  (`KismetArrayLibrary.Array_Clear` (`self.HittedActor`))
  (`self.Spawn Shuriken Projectile`))

(event `self.MeleeBox.OnComponentBeginOverlap`
  (params (OverlappedComponent :type "PrimitiveComponent Object Reference") (OtherActor :type "Actor Object Reference") (OtherComp :type "PrimitiveComponent Object Reference") (OtherBodyIndex :type Integer) (bFromSweep :type Boolean) (SweepResult :type "HitResult Structure (by ref)"))
  ;[1 0.3906 0.3906] Melee Attack
  ;;[1 1 1] On Hit Logic Normal
  (`self.MeleeHitLogic` OtherActor OtherComp))

(event `self.SpinCapsule.OnComponentBeginOverlap`
  (params (OverlappedComponent :type "PrimitiveComponent Object Reference") (OtherActor :type "Actor Object Reference") (OtherComp :type "PrimitiveComponent Object Reference") (OtherBodyIndex :type Integer) (bFromSweep :type Boolean) (SweepResult :type "HitResult Structure (by ref)"))
  ;[1 0.3906 0.3906] Melee Attack
  ;;[1 1 1] On Hit Logic Spin
  (`self.MeleeHitLogic` OtherActor OtherComp))

(event `self.ReceiveBeginPlay`
  ;[1 1 1] Begin Play Create UI
  (bind _returnvalue (`|CreateWidget` "/Game/UI/UI_Base.UI_Base_C"))
  (bind _output_get (set `self.Widget` _returnvalue))
  (`UserWidget.AddToViewport` _output_get 0)
  (bind _returnvalue_2 (`|GetDataTableRow` "/Game/Blueprint/Stats_DataTable.Stats_DataTable" "PlayerInitialHealth")
    (:`then`
      (set `self.Health` (break `/Game/Blueprint/Stats_Struct` _returnvalue_2)))))

(event `self.ReceiveTick`
  (params (DeltaSeconds :type "Float (single-precision)"))
  ;[1 1 1] Look at Cursor
  (`/Engine/EditorBlueprintResources/StandardMacros.Gate` false :!label _label_2
    (:`Exit`
      (`|ExecutionSequence`
        (:`then_0`
          (`self.RotateToCursor`))
        (:`then_1`
          (`self.UpdateTimer`))
        (:`then_2`
          (for _array_element (`self.ShurikenEffect`)
            (`KismetSystemLibrary.PrintString` (`|GetEnumeratorNameAsString` _array_element) true true (struct :`G` 0.66 :`B` 1.0 :`A` 1.0) 0.01)))))))

(event `StopTick`
  ;[1 1 1] Look at Cursor
  (goto _label_2 :!via `Close`))

(event `/Game/Blueprint/BPI_Damage.DamageInput`
  (params (Damages :type "Float (single-precision)") (AttackType :type "/Game/Blueprint/EShurikenEffects Enum" :default "NewEnumerator0"))
  ;[1 1 1] Receive Dmg Logic
  (bind _isdead (`self.UpdateHealth` Damages))
  (if _isdead
    (`self.Death`)))

(event `AddShurikenEffect`
  (params (Effect :type "/Game/Blueprint/EShurikenEffects Enum" :default "NewEnumerator0"))
  ;[1 1 1] Set Shuriken Effects
  (`KismetArrayLibrary.Array_AddUnique` (`self.ShurikenEffect`) Effect))

(event `RemoveShurikenEffect`
  (params (Effect :type "/Game/Blueprint/EShurikenEffects Enum" :default "NewEnumerator0"))
  ;[1 1 1] Set Shuriken Effects
  (`KismetArrayLibrary.Array_RemoveItem` (`self.ShurikenEffect`) Effect))

(event `InputAxisKey|MouseWheelAxis`
  (params (AxisValue :type "Float (single-precision)"))
  (bind _springarm (`self.SpringArm`))
  ;[1 1 1] ZoomIn ZoomOut
  (if (!= AxisValue 0.0)
    (set `SpringArmComponent.TargetArmLength` (+ (* AxisValue -20.0) (`SpringArmComponent.TargetArmLength` _springarm)) _springarm)))

(fn `Dash`
  (bind _returnvalue (`self.GetInputAxisValue`))
  (bind _returnvalue_2 (`self.GetInputAxisValue`))
  (bind _returnvalue_3 (- (`SceneComponent.K2_GetComponentLocation` (`self.CapsuleComponent`)) (0.0 0.0 30.0)))
  (bind _returnvalue_4 (`|GetDataTableRow` "/Game/Blueprint/Stats_DataTable.Stats_DataTable" "DashBaseDistance")
    (:`then`
      (bind _returnvalue_5 (+ _returnvalue_3 (* (`KismetMathLibrary.MakeVector` (.x (select `bool` (and (== _returnvalue_2 0.0) (== _returnvalue 0.0)) :`false` (`KismetMathLibrary.MakeVector` _returnvalue_2 _returnvalue) :`true` (`SceneComponent.GetForwardVector` (`self.CapsuleComponent`)))) (.y (select `bool` (and (== _returnvalue_2 0.0) (== _returnvalue 0.0)) :`false` (`KismetMathLibrary.MakeVector` _returnvalue_2 _returnvalue) :`true` (`SceneComponent.GetForwardVector` (`self.CapsuleComponent`))))) (break `/Game/Blueprint/Stats_Struct` _returnvalue_4))))
      (bind (_outhit _returnvalue_6) (`KismetSystemLibrary.LineTraceSingleForObjects` _returnvalue_3 _returnvalue_5 (`|MakeArray` "ObjectTypeQuery1" :!type "EObjectTypeQuery Enum")))
      (`self.K2_TeleportTo` (select `bool` _returnvalue_6 :`false` _returnvalue_5 :`true` (`.Location` (`GameplayStatics.BreakHitResult` _outhit))) (`SceneComponent.K2_GetComponentRotation` (`self.CapsuleComponent`)))
      (return))))

(fn `Death`
  (`Widget.SetVisibility` (`/Game/UI/UI_Base.GameOver` (`self.Widget`)) "Visible")
  (`self.DisableInput` (`GameplayStatics.GetPlayerController` 0))
  (bind _asanim_bp_base (cast `/Game/Blueprint/AnimBP_Base` (`SkeletalMeshComponent.GetAnimInstance` (`self.Mesh`))))
  (`/Game/Blueprint/AnimBP_Base.Death` _asanim_bp_base)
  (`self.StopTick`))

(fn `RotateToCursor`
  (bind (_returnvalue_roll _returnvalue_pitch _returnvalue_yaw) (`KismetMathLibrary.BreakRotator` (`KismetMathLibrary.FindLookAtRotation` (`SceneComponent.K2_GetComponentLocation` (`self.CapsuleComponent`)) (`.Location` (`GameplayStatics.BreakHitResult` (`PlayerController.GetHitResultUnderCursorForObjects` (`GameplayStatics.GetPlayerController` 0) (`|MakeArray` "ObjectTypeQuery7" :!type "EObjectTypeQuery Enum") true))))))
  (`SceneComponent.K2_SetWorldRotation` (`self.CapsuleComponent`) (`KismetMathLibrary.MakeRotator` 0.0 0.0 _returnvalue_yaw) false false)
  (set `self.LookAtDirection` _returnvalue_yaw))

(fn `Spawn Shuriken Projectile`
  ;[1 1 1] Spawn Projectile at Location
  (bind _returnvalue (`|SpawnActorFromClass` "/Game/Blueprint/BP_Shuriken.BP_Shuriken_C" (`KismetMathLibrary.MakeTransform` (`SceneComponent.K2_GetComponentLocation` (`self.CapsuleComponent`)) (`KismetMathLibrary.Conv_VectorToRotator` (`SceneComponent.GetForwardVector` (`self.CapsuleComponent`)))) "AlwaysSpawn" "OverrideRootScale" null null))
  ;[1 1 1] Set Shuriken Component
  (`/Engine/EditorBlueprintResources/StandardMacros.IsValid` _returnvalue
    (:`Is Valid`
      (set `/Game/Blueprint/BP_Shuriken.Effects` (`self.ShurikenEffect`) _returnvalue))))

(fn `UpdateScore`
  (params (Points :type Integer))
  (bind _output_get (set `self.Score` (+ (`self.Score`) Points)))
  (`TextBlock.SetText` (`/Game/UI/UI_Base.ScoreCounter` (`self.Widget`)) (`KismetTextLibrary.Conv_IntToText` _output_get))
  (return))

(fn `UserConstructionScript`
  (bind _returnvalue (`|GetDataTableRow` "/Game/Blueprint/Stats_DataTable.Stats_DataTable" "PlayerBaseSpeed")
    (:`then`
      (set `CharacterMovementComponent.MaxWalkSpeed` (break `/Game/Blueprint/Stats_Struct` _returnvalue) (`self.CharacterMovement`)))))