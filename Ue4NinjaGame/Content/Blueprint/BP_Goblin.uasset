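; BP_Goblin is a short-lived wandering monster that drops a random ability pickup when killed.
; The construction script sets lifespan, walk speed and health from a stats DataTable.
; It loops AI moves to random navigable points within the BP_BaseSpawner's sphere.
; DamageInput lowers health, feeds the health ratio to a crack material parameter, then plays hit effects or handles death; any destruction, including expiry, spawns an emitter.
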(event `self.ReceiveBeginPlay`
  ;[1 1 1] Begin Play
  (bind _returnvalue (`GameplayStatics.GetActorOfClass` "/Game/Blueprint/BP_BaseSpawner.BP_BaseSpawner_C"))
  (`/Engine/EditorBlueprintResources/StandardMacros.IsValid` _returnvalue
    (:`Is Valid`
      (set `self.Spawn Sphere` (`/Game/Blueprint/BP_BaseSpawner.Block_Shpere` _returnvalue))
      (`self.WalkToRandomDest`)
      ;[1 1 1] Death Particle Effect
      (add `self.OnDestroyed` (delegate `DestroyEmitter`)))))

(event `DestroyEmitter` :!signature `self.OnDestroyed`
  (params (DestroyedActor :type "Actor Object Reference"))
  ;[1 1 1] Death Particle Effect
  (`GameplayStatics.SpawnEmitterAtLocation` "/Game/MarketPlace/AdvancedMagicFX12/particles/P_ky_hit.P_ky_hit" (`SceneComponent.K2_GetComponentLocation` (`self.CapsuleComponent`))))

(event `WalkToRandomDest`
  (bind _spawn_sphere (`self.Spawn Sphere`))
  ;[1 1 1] Walk on Random Location
  (bind _randomlocation (`NavigationSystemV1.K2_GetRandomLocationInNavigableRadius` (`SceneComponent.K2_GetComponentLocation` _spawn_sphere) (`SphereComponent.SphereRadius` _spawn_sphere) null null))
  (`|AIMoveTo` self _randomlocation null
    (:`OnSuccess`
      _)
    (:`OnFail`
      _))
  (`self.WalkToRandomDest`))

(event `/Game/Blueprint/BPI_Damage.DamageInput`
  (params (Damages :type "Float (single-precision)") (AttackType :type "/Game/Blueprint/EShurikenEffects Enum" :default "NewEnumerator0"))
  (bind _capsulecomponent (`self.CapsuleComponent`))
  ;[1 1 1] On Hit Logic
  (if (not (`self.IsDead`))
    (bind _output_get (set `self.Health` (- (`self.Health`) Damages)))
    ;;[1 0.2384 0.873] Update Visual Monster Health
    (bind _returnvalue (`|GetDataTableRow` "/Game/Blueprint/Stats_DataTable.Stats_DataTable" "GoblinBaseHealth")
      (:`then`
        (`MeshComponent.SetScalarParameterValueOnMaterials` (`self.StaticMesh`) "CracksIntensity" (/ (`self.Health`) (break `/Game/Blueprint/Stats_Struct` _returnvalue)))
        (if (<= _output_get 0.0)
          (set `self.IsDead` true)
          ;[1 1 1] On Death Logic
          (`|SpawnActorFromClass` "/Game/Blueprint/AltShuriken/BP_AbilityPickUp_Random.BP_AbilityPickUp_Random_C" (`KismetMathLibrary.MakeTransform` (- (`SceneComponent.K2_GetComponentLocation` (`self.CapsuleComponent`)) (`KismetMathLibrary.MakeVector` 0.0 0.0 (`CapsuleComponent.CapsuleHalfHeight` (`self.CapsuleComponent`))))) "Undefined" "OverrideRootScale" null null)
          (`KismetSystemLibrary.Delay` 0.0) ; To have time to run code before
          (`self.K2_DestroyActor`)
          (else
            ;[1 1 1] Hit Particle Effect
            (`NiagaraFunctionLibrary.SpawnSystemAttached` "/Game/Stylized_VFX_StPack/Particles/UPDATE_1_3/P_Web_Hit_01.P_Web_Hit_01" _capsulecomponent "None" (`KismetMathLibrary.MakeVector` (`CapsuleComponent.CapsuleRadius` _capsulecomponent)) (struct) "KeepRelativeOffset" true)))))))

(fn `UserConstructionScript`
  (bind _returnvalue (`|GetDataTableRow` "/Game/Blueprint/Stats_DataTable.Stats_DataTable" "GoblinBaseDuration")
    (:`then`
      (`self.SetLifeSpan` self (break `/Game/Blueprint/Stats_Struct` _returnvalue))
      (bind _returnvalue_2 (`|GetDataTableRow` "/Game/Blueprint/Stats_DataTable.Stats_DataTable" "GoblinBaseSpeed")
        (:`then`
          (set `CharacterMovementComponent.MaxWalkSpeed` (break `/Game/Blueprint/Stats_Struct` _returnvalue_2) (`self.CharacterMovement`))
          (bind _returnvalue_3 (`|GetDataTableRow` "/Game/Blueprint/Stats_DataTable.Stats_DataTable" "GoblinBaseHealth")
            (:`then`
              (set `self.Health` (break `/Game/Blueprint/Stats_Struct` _returnvalue_3)))))))))